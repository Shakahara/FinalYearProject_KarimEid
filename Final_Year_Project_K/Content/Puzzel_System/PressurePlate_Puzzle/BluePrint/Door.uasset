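; Puzzle door that opens while enough pressure switches are active and closes when the count drops below the required number.
; SwitchActivated and SwitchDeactivated adjust an active switch counter and compare it to PressureSwitchNeeded, playing or reversing the DoorAnimation timeline.
; The timeline drives the door's relative Z location.
; The sliding sound plays only on activations that meet the threshold, at world origin rather than at the door.
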(event Custom|SwitchActivated
  (Math|Integer|IncrementInt (Variables|Default|GetPressureSwitchActive)
    (:%20%20
      (if (>= (Variables|Default|GetPressureSwitchActive) (Variables|Default|GetPressureSwitchNeeded))
        (Audio|PlaySoundatLocation "/Game/Puzzel_System/Sounds_Export/Sliding_door.Sliding_door" "0, 0, 0" "0, 0, 0" 1.0 1.0 0.0 0 0 0)
        (bind _doorpos (Timeline|Door%20Animation Play)
          (:Update
            (Transformation|SetRelativeLocation (Variables|Default|GetDoor) (Math|Vector|MakeVector 0.0 0.0 _doorpos) false false)))
        (else
          (Timeline|Door%20Animation Reverse))))))

(event Custom|SwitchDeactivated
  (Math|Integer|DecrementInt (Variables|Default|GetPressureSwitchActive)
    (:%20%20
      (if (>= (Variables|Default|GetPressureSwitchActive) (Variables|Default|GetPressureSwitchNeeded))
        (bind _doorpos (Timeline|Door%20Animation Play)
          (:Update
            (Transformation|SetRelativeLocation (Variables|Default|GetDoor) (Math|Vector|MakeVector 0.0 0.0 _doorpos) false false)))
        (else
          (Timeline|Door%20Animation Reverse))))))

(event EventBeginPlay)

(fn ConstructionScript)